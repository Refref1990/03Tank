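; BP_Tank is a player-controlled tank whose input graph handles camera rotation and firing.
; On BeginPlay it passes the barrel and turret components to the Aiming component and the barrel to the tank itself.
; Azimuth input yaws the Scene component, attitude input pitches the SpringArm, and Fire calls Spara, which is defined outside these graphs.
; Blueprint nodes for spawning a projectile and playing its sound are left unconnected.
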(event EventBeginPlay)

(event Collision|EventActorBeginOverlap
  (params (OtherActor :type Actor%20Object%20Reference)))

(event EventTick
  (params (DeltaSeconds :type Float%20%28single-precision%29)))

(event EventBeginPlay
  (bind _aiming (Variables|Default|GetAiming))
  (Class|AimingComponent|SetCannone _aiming (Variables|Default|GetBarrel%202.0))
  (Class|AimingComponent|SetTorre _aiming (Variables|Default|GetTurret%202.0))
  (Class|TankC|SetCannone (Variables|Default|GetBarrel%202.0)))

(event Input|ActionEvents|InputActionFire
  (params (Key :type Key%20Structure :default "None"))
  (:Pressed
    (Class|TankC|Spara)))

(event Input|AxisEvents|InputAxisMoveAzimuth
  (params (AxisValue :type Float%20%28single-precision%29))
  (Transformation|AddLocalRotation (Variables|Default|GetScene) (Math|Rotator|MakeRotator 0.0 0.0 AxisValue) false false))

(event Input|AxisEvents|InputAxisMoveAttitude
  (params (AxisValue :type Float%20%28single-precision%29))
  (Transformation|AddLocalRotation (Variables|Default|GetSpringArm) (Math|Rotator|MakeRotator 0.0 AxisValue 0.0) false false))

(fn ConstructionScript)